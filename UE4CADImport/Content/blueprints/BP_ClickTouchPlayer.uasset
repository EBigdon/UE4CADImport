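; Click/touch player Blueprint holding experimental camera-control logic; none of its event-graph chains has a connected trigger, so none runs.
; Gate and Delay loops nudge EditRotation or step EditVector along fixed axes or through CalculateRotation, a yaw-based offset that also prints debug output.
; Other chains apply these values to every CameraActor, positioning it relative to this actor and snapping or interpolating its rotation.
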(fn `calculateRotation`
  (params (vector :type "Vector Structure"))
  (returns (NewParam :type "Vector Structure"))
  (bind (_editrotation_roll _editrotation_pitch _editrotation_yaw) (`KismetMathLibrary.BreakRotator` (`self.editRotation`)))
  (bind _returnvalue (+ (mod (* 1000 _editrotation_yaw) 360.0) 1.0))
  (bind _returnvalue_2 (`KismetMathLibrary.DegSin` _returnvalue))
  (bind _returnvalue_3 (* (`KismetMathLibrary.MakeVector` (* (+ (* vector_X _returnvalue_2) (* vector_X _returnvalue)) 0.02) (* (+ (* vector_Y _returnvalue_2) (* vector_Y _returnvalue)) 0.02)) (-1.0 -1.0 -1.0)))
  (`KismetSystemLibrary.PrintString` (`KismetStringLibrary.Conv_VectorToString` _returnvalue_3))
  (return _returnvalue_3))

(fn `modulo`
  (params (param :type Integer) (modulo_operator :type Integer))
  (returns (rest :type Integer))
  (return (- param (* (/ param modulo_operator) modulo_operator))))

(fn `UserConstructionScript`)